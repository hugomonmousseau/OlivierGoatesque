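; BP_glaive is a glaive item that the first-person character can pick up once through an Interact event.
; Interact casts the triggering actor to BP_FirstPersonCharacter, notifies it of the pickup and attaches a component to its GlaiveSocket, snapping location while keeping relative rotation and scale.
; A GlaiveIsTaken flag blocks repeat pickups, and the Box component is deactivated afterwards.
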(event EventInteract
  (params (Acor%20Triggering%20Interact :type Actor%20Object%20Reference))
  (if (not (Variables|Default|GetGlaiveIsTaken))
    (bind _asbp_first_person_character (Utilities|Casting|CastToBP_FirstPersonCharacter Acor%20Triggering%20Interact))
    (Default|ItemHasBeenPickUp _asbp_first_person_character self)
    (Transformation|AttachComponentToComponent (Variables|/Game/FirstPerson/Blueprints/BP_FirstPersonCharacter.BP_FirstPersonCharacter_C|GetglaiveSocket _asbp_first_person_character) "None" "SnapToTarget" "KeepRelative" "KeepRelative" true)
    (Variables|Default|SetGlaiveIsTaken true)
    (Components|Activation|SetActive (Variables|Default|GetBox) false false)))

(fn ConstructionScript
  (|CallParentFunction))