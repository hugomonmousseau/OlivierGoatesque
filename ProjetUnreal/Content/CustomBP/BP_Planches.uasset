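; BP_Planches is an interactable wood planks resource that the player harvests with the sword.
; On Interact, it casts the triggering actor to BP_FirstPersonCharacter and checks whether the sword is in hand.
; If it is, it adds StickQuantity to the character's StickQ, destroys itself and prints a hardcoded "+2 woods" message.
; Otherwise, it only prints a hint to use the sword.
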(event EventInteract
  (params (Acor%20Triggering%20Interact :type Actor%20Object%20Reference))
  (bind _asbp_first_person_character (Utilities|Casting|CastToBP_FirstPersonCharacter Acor%20Triggering%20Interact))
  (if (Variables|/Game/FirstPerson/Blueprints/BP_FirstPersonCharacter.BP_FirstPersonCharacter_C|GetIsSwordInHand _asbp_first_person_character)
    (bind _asbp_first_person_character_2 (Utilities|Casting|CastToBP_FirstPersonCharacter Acor%20Triggering%20Interact))
    (Variables|/Game/FirstPerson/Blueprints/BP_FirstPersonCharacter.BP_FirstPersonCharacter_C|SetStickQ _asbp_first_person_character_2 (+ (Variables|/Game/FirstPerson/Blueprints/BP_FirstPersonCharacter.BP_FirstPersonCharacter_C|GetStickQ _asbp_first_person_character_2) (Variables|Default|GetStickQuantity)))
    (Actor|DestroyActor)
    (Development|PrintString "+2 woods" true true "(R=0.274510,G=0.180392,B=0.047059,A=1.000000)")
    (else
      (Development|PrintString "use sword"))))

(fn ConstructionScript
  (|CallParentFunction))