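; BP_ClothesLine is a harvestable clothesline that the first-person character dismantles in stages for crafting-style resources.
; Interact requires the sword in hand, otherwise it prints a hint to use it.
; A Step counter drives each stage, swapping the static mesh and ItemName while incrementing the character's cloth, then rope, then stick count.
; The final stage destroys the actor, and each pickup is reported with a colored PrintString.
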(event EventInteract
  (params (Acor%20Triggering%20Interact :type Actor%20Object%20Reference))
  (bind _asbp_first_person_character (Utilities|Casting|CastToBP_FirstPersonCharacter Acor%20Triggering%20Interact))
  (if (Variables|/Game/FirstPerson/Blueprints/BP_FirstPersonCharacter.BP_FirstPersonCharacter_C|GetIsSwordInHand _asbp_first_person_character)
    (Transformation|SetWorldScale3D (Variables|Default|GetMesh) "100.000000,100.000000,100.000000")
    (if (== (Variables|Default|GetStep) 1)
      (Components|StaticMesh|SetStaticMesh (Variables|Default|GetMesh) (Variables|Default|GetMeshWithRope))
      (Variables|Default|SetStep 2)
      (bind _asbp_first_person_character_2 (Utilities|Casting|CastToBP_FirstPersonCharacter Acor%20Triggering%20Interact))
      (bind _result (Math|Integer|IncrementInt (Variables|/Game/FirstPerson/Blueprints/BP_FirstPersonCharacter.BP_FirstPersonCharacter_C|GetTissuQ _asbp_first_person_character_2))
        (:%20%20
          (Variables|/Game/FirstPerson/Blueprints/BP_FirstPersonCharacter.BP_FirstPersonCharacter_C|SetTissuQ _asbp_first_person_character_2 _result)
          (Variables|Default|SetItemName "rope")
          (Development|PrintString "+1 sheet" true true "(R=0.639216,G=0.180392,B=0.105882,A=1.000000)")))
      (elif (== (Variables|Default|GetStep) 2)
        (Components|StaticMesh|SetStaticMesh (Variables|Default|GetMesh) (Variables|Default|GetMeshWithNothing))
        (bind _asbp_first_person_character_3 (Utilities|Casting|CastToBP_FirstPersonCharacter Acor%20Triggering%20Interact))
        (bind _result_2 (Math|Integer|IncrementInt (Variables|/Game/FirstPerson/Blueprints/BP_FirstPersonCharacter.BP_FirstPersonCharacter_C|GetRopeQ _asbp_first_person_character_3))
          (:%20%20
            (Variables|/Game/FirstPerson/Blueprints/BP_FirstPersonCharacter.BP_FirstPersonCharacter_C|SetRopeQ _asbp_first_person_character_3 _result_2)
            (Variables|Default|SetItemName "sticks")
            (Variables|Default|SetStep 3)
            (Development|PrintString "+1 rope" true true "(R=0.639216,G=0.462745,B=0.168627,A=1.000000)")))
        (else
          (bind _asbp_first_person_character_4 (Utilities|Casting|CastToBP_FirstPersonCharacter Acor%20Triggering%20Interact))
          (bind _result_3 (Math|Integer|IncrementInt (Variables|/Game/FirstPerson/Blueprints/BP_FirstPersonCharacter.BP_FirstPersonCharacter_C|GetStickQ _asbp_first_person_character_4))
            (:%20%20
              (Variables|/Game/FirstPerson/Blueprints/BP_FirstPersonCharacter.BP_FirstPersonCharacter_C|SetStickQ _asbp_first_person_character_4 _result_3)
              (Actor|DestroyActor)
              (Development|PrintString "+1 wood" true true "(R=0.274510,G=0.180392,B=0.047059,A=1.000000)"))))))
    (else
      (Development|PrintString "use sword"))))

(fn ConstructionScript
  (|CallParentFunction))