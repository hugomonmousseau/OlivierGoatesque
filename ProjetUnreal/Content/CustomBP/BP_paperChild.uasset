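; A paper page the player picks up by interacting, then carries in view as an inspectable item.
; Interact notifies the first-person character and attaches the page to its inspect socket, once only.
; While held, Tick blends its position between that socket and the character's MapPosition by camera pitch, tilting it further when looking down.
; BeginPlay applies the page's material to its plane mesh.
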(event EventTick
  (params (DeltaSeconds :type Float%20%28single-precision%29))
  (bind _defaultsceneroot (Variables|Default|GetDefaultSceneRoot))
  (if (Variables|Default|GetPageIsTaken)
    (Utilities|FlowControl|Sequence
      (:then_0
        (bind _asbp_first_person_character (Utilities|Casting|CastToBP_FirstPersonCharacter (Game|GetPlayerCharacter 0)))
        (if (< (.pitch (Transformation|GetWorldRotation (Variables|/Game/FirstPerson/Blueprints/BP_FirstPersonCharacter.BP_FirstPersonCharacter_C|GetFirstPersonCamera _asbp_first_person_character))) 0.0)
          (Transformation|SetWorldRotation _defaultsceneroot (Math|Rotator|MakeRotator (.roll (Transformation|GetWorldRotation (Variables|/Game/FirstPerson/Blueprints/BP_FirstPersonCharacter.BP_FirstPersonCharacter_C|GetItemInscpectSocket _asbp_first_person_character))) (+ (* (.pitch (Transformation|GetWorldRotation (Variables|/Game/FirstPerson/Blueprints/BP_FirstPersonCharacter.BP_FirstPersonCharacter_C|GetFirstPersonCamera _asbp_first_person_character))) -0.3) -1e+02) (.yaw (Transformation|GetWorldRotation (Variables|/Game/FirstPerson/Blueprints/BP_FirstPersonCharacter.BP_FirstPersonCharacter_C|GetItemInscpectSocket _asbp_first_person_character)))) false false)
          (else
            (Transformation|SetWorldRotation _defaultsceneroot (Math|Rotator|MakeRotator (.roll (Transformation|GetWorldRotation (Variables|/Game/FirstPerson/Blueprints/BP_FirstPersonCharacter.BP_FirstPersonCharacter_C|GetItemInscpectSocket _asbp_first_person_character))) -9e+01 (.yaw (Transformation|GetWorldRotation (Variables|/Game/FirstPerson/Blueprints/BP_FirstPersonCharacter.BP_FirstPersonCharacter_C|GetItemInscpectSocket _asbp_first_person_character)))) false false)))
        (Transformation|SetWorldLocation (Variables|Default|GetDefaultSceneRoot) (+ (* (Transformation|GetWorldLocation (Variables|/Game/FirstPerson/Blueprints/BP_FirstPersonCharacter.BP_FirstPersonCharacter_C|GetMapPosition _asbp_first_person_character)) (/ (+ (.pitch (Transformation|GetWorldRotation (Variables|/Game/FirstPerson/Blueprints/BP_FirstPersonCharacter.BP_FirstPersonCharacter_C|GetFirstPersonCamera _asbp_first_person_character))) 9e+01) 1.8e+02)) (* (Transformation|GetWorldLocation (Variables|/Game/FirstPerson/Blueprints/BP_FirstPersonCharacter.BP_FirstPersonCharacter_C|GetItemInscpectSocket _asbp_first_person_character)) (- 1.0 (/ (+ (.pitch (Transformation|GetWorldRotation (Variables|/Game/FirstPerson/Blueprints/BP_FirstPersonCharacter.BP_FirstPersonCharacter_C|GetFirstPersonCamera _asbp_first_person_character))) 9e+01) 1.8e+02)))) false false)))))

(event EventBeginPlay
  (Rendering|Material|SetMaterial (Variables|Default|GetPlane) 0 (Variables|Default|GetMaterial)))

(event EventInteract
  (params (Acor%20Triggering%20Interact :type Actor%20Object%20Reference))
  (if (not (Variables|Default|GetPageIsTaken))
    (bind _asbp_first_person_character (Utilities|Casting|CastToBP_FirstPersonCharacter Acor%20Triggering%20Interact))
    (Default|ItemHasBeenPickUp _asbp_first_person_character self)
    (Transformation|AttachComponentToComponent (Variables|/Game/FirstPerson/Blueprints/BP_FirstPersonCharacter.BP_FirstPersonCharacter_C|GetItemInscpectSocket _asbp_first_person_character) "None" "SnapToTarget" "KeepRelative" "KeepRelative" true)
    (Variables|Default|SetPageIsTaken true)))

(fn ConstructionScript
  (|CallParentFunction))