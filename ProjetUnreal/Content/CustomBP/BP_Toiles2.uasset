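; BP_Toiles2 is a two-stage harvestable interactable that yields cloth and then sticks to the first-person character.
; Interacting requires a sword in hand; otherwise it prints a "use sword" message.
; The first interaction adds cloth to the character, swaps and rescales the mesh, and relabels the look-at prompt for sticks.
; The second adds sticks and destroys the actor, with each pickup reported through a printed message.
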(event EventInteract
  (params (Acor%20Triggering%20Interact :type Actor%20Object%20Reference))
  (bind _asbp_first_person_character (Utilities|Casting|CastToBP_FirstPersonCharacter Acor%20Triggering%20Interact))
  (if (Variables|/Game/FirstPerson/Blueprints/BP_FirstPersonCharacter.BP_FirstPersonCharacter_C|GetIsSwordInHand _asbp_first_person_character)
    (if (== (Variables|Default|GetStep) 1)
      (Transformation|SetRelativeScale3D (Variables|Default|GetMesh) "100.000000,100.000000,100.000000")
      (Components|StaticMesh|SetStaticMesh (Variables|Default|GetMesh) (Variables|Default|GetNew%20Mesh))
      (bind _asbp_first_person_character_2 (Utilities|Casting|CastToBP_FirstPersonCharacter Acor%20Triggering%20Interact))
      (Variables|/Game/FirstPerson/Blueprints/BP_FirstPersonCharacter.BP_FirstPersonCharacter_C|SetTissuQ _asbp_first_person_character_2 (+ (Variables|/Game/FirstPerson/Blueprints/BP_FirstPersonCharacter.BP_FirstPersonCharacter_C|GetTissuQ _asbp_first_person_character_2) (Variables|Default|GetTissusObtenus)))
      (Variables|Default|SetStep 2)
      (Variables|Default|SetItemName "sticks")
      (Variables|Default|SetLookAtActionName "Take")
      (Development|PrintString "+3 sheets" true true "(R=0.639216,G=0.180392,B=0.105882,A=1.000000)")
      (elif (== (Variables|Default|GetStep) 2)
        (bind _asbp_first_person_character_3 (Utilities|Casting|CastToBP_FirstPersonCharacter Acor%20Triggering%20Interact))
        (Variables|/Game/FirstPerson/Blueprints/BP_FirstPersonCharacter.BP_FirstPersonCharacter_C|SetStickQ _asbp_first_person_character_3 (+ (Variables|/Game/FirstPerson/Blueprints/BP_FirstPersonCharacter.BP_FirstPersonCharacter_C|GetStickQ _asbp_first_person_character_3) (Variables|Default|GetBatonObtenus)))
        (Actor|DestroyActor)
        (Development|PrintString "+2 woods" true true "(R=0.274510,G=0.180392,B=0.047059,A=1.000000)")))
    (else
      (Development|PrintString "use sword"))))

(fn ConstructionScript
  (|CallParentFunction))