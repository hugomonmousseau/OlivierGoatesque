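; BP_InteractableDoor is a door that swings open and closed on interaction, optionally locked behind a key.
; When locked, Interact checks the first-person character's Inventory for KeyID and clears the lock without consuming the key or opening the door.
; When unlocked, a FlipFlop alternates playing and reversing a timeline that drives the door's yaw.
; IsOpenAtStart triggers that same toggle on BeginPlay, bypassing the lock.
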(event EventBeginPlay
  (if (Variables|Default|GetIsOpenAtStart)
    (Utilities|FlowControl|FlipFlop
      (:A
        (bind _tr_animatedoortrack (Timeline|TL_AnimateDoor Play)
          (:Update
            (Transformation|SetRelativeRotation (Variables|Default|GetDoor) (Math|Rotator|MakeRotator 0.0 0.0 _tr_animatedoortrack) false false))))
      (:B
        (Timeline|TL_AnimateDoor Reverse)))))

(event EventInteract
  (params (Acor%20Triggering%20Interact :type Actor%20Object%20Reference))
  (if (Variables|Default|GetIsKeyNeeded)
    (bind _asbp_first_person_character (Utilities|Casting|CastToBP_FirstPersonCharacter Acor%20Triggering%20Interact))
    (if (.ReturnValue (Utilities|Map|Find (Variables|/Game/FirstPerson/Blueprints/BP_FirstPersonCharacter.BP_FirstPersonCharacter_C|GetInventory _asbp_first_person_character) (Variables|Default|GetKeyID)))
      (if (> (.Value (Utilities|Map|Find (Variables|/Game/FirstPerson/Blueprints/BP_FirstPersonCharacter.BP_FirstPersonCharacter_C|GetInventory _asbp_first_person_character) (Variables|Default|GetKeyID))) 0)
        (Variables|Default|SetIsKeyNeeded false)))
    (else
      (Utilities|FlowControl|FlipFlop
        (:A
          (bind _tr_animatedoortrack (Timeline|TL_AnimateDoor Play)
            (:Update
              (Transformation|SetRelativeRotation (Variables|Default|GetDoor) (Math|Rotator|MakeRotator 0.0 0.0 _tr_animatedoortrack) false false))))
        (:B
          (Timeline|TL_AnimateDoor Reverse))))))

(fn ConstructionScript
  (|CallParentFunction))