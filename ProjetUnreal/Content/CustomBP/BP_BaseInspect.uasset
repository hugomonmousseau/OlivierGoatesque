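; BP_BaseInspect is a base actor for items the first-person player can pick up and inspect by rotating them.
; Interact hands input from the player character to the item and snaps it to the character's inspect socket component.
; While inspecting, IA_Look rotates the item in pitch and yaw.
; IA_Interact ends inspection, returning input to the player and detaching the item back to the transform saved at BeginPlay.
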(event Input|EnhancedActionEvents|EnhancedInputActionIA_Interact
  (params (ActionValue :type Boolean) (ElapsedSeconds :type Float%20%28double-precision%29) (TriggeredSeconds :type Float%20%28double-precision%29) (InputAction :type Input%20Action%20Object%20Reference :default "/Game/FirstPerson/Input/Actions/IA_Interact.IA_Interact"))
  (CallFunction|StopInspection))

(event Input|EnhancedActionEvents|EnhancedInputActionIA_Look
  (params (ActionValue :type Vector%202D%20Structure) (ElapsedSeconds :type Float%20%28double-precision%29) (TriggeredSeconds :type Float%20%28double-precision%29) (InputAction :type Input%20Action%20Object%20Reference :default "/Game/FirstPerson/Input/Actions/IA_Look.IA_Look"))
  (bind (_x _y) (Math|Vector2D|BreakVector2D ActionValue))
  (Transformation|SetActorRotation (Math|Rotator|CombineRotators (Transformation|GetActorRotation) (Math|Rotator|MakeRotator 0.0 (* _y 3.0) (* _x -3.0)))))

(event EventInteract
  (params (Acor%20Triggering%20Interact :type Actor%20Object%20Reference))
  (bind _asbp_first_person_character (Utilities|Casting|CastToBP_FirstPersonCharacter Acor%20Triggering%20Interact))
  (Variables|Default|SetBP_Player _asbp_first_person_character)
  (CallFunction|StartInspection))

(event EventBeginPlay
  (Variables|Default|SetInitTransform (Transformation|GetActorTransform)))

(fn ConstructionScript
  (|CallParentFunction))

(fn StartInspection
  (bind _returnvalue (Game|GetPlayerController 0))
  (bind _bp_player (Variables|Default|GetBP_Player))
  (Input|DisableInput _bp_player _returnvalue)
  (Input|EnableInput _returnvalue)
  (Transformation|AttachComponentToComponent (Variables|/Game/FirstPerson/Blueprints/BP_FirstPersonCharacter.BP_FirstPersonCharacter_C|GetItemInscpectSocket _bp_player) "None" "SnapToTarget" "SnapToTarget" "KeepWorld" true))

(fn StopInspection
  (bind _returnvalue (Game|GetPlayerController 0))
  (Input|DisableInput _returnvalue)
  (Input|EnableInput (Variables|Default|GetBP_Player) _returnvalue)
  (Transformation|DetachFromActor "KeepRelative" "KeepRelative" "KeepRelative")
  (Transformation|SetActorTransform (Variables|Default|GetInitTransform)))